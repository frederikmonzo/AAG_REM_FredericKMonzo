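; Erick2 is the player character: movement, hitscan shooting, grenades, two aimed portals, an outline pulse, pause menu and HUD compass.
; E flips gravity by rolling actor and camera, applying upward force through a Tick-fed gate, and inverting input and jump.
; A looping timer traces overhead to set a Gravedad flag.
; Custom events handle camera recentering and grenade arc preview, but nothing here calls them; the grenade charge loop never runs.
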(event Custom|CustomEvent_Camara
  (params (DeltaSeconds :type Float%20%28single-precision%29))
  (bind _returnvalue (Math|Rotator|MakeRotator 0.0 9e+01 0.0))
  (bind _returnvalue_2 (Pawn|GetControlRotation :!class /Script/Engine.Pawn))
  (bind _mesh (Variables|Character|GetMesh))
  (bind _returnvalue_3 (Transformation|GetWorldRotation _mesh))
  (bind _returnvalue_4 (Math|Rotator|CombineRotators _returnvalue_3 _returnvalue))
  (bind _returnvalue_5 (Math|Rotator|Delta(Rotator) _returnvalue_4 _returnvalue_2))
  (bind _pitch (Math|Rotator|BreakRotator _returnvalue_5))
  ;[1 1 1] Formateo de Camara
  (if (Variables|Default|GetCamaraFormateo)
    (Pawn|Input|AddControllerYawInput (* DeltaSeconds _pitch (Variables|Default|GetCamaraRotacion)))
    (if (< (Math|Float|Absolute(Float) _pitch) 2.0)
      (Variables|Default|SetCamaraFormateo false))))

(event Custom|CustomEvent_Granada
  (params (DeltaSeconds :type Float%20%28single-precision%29))
  (bind _realeasedgranada (Variables|Default|GetRealeasedGranada))
  (bind _granada (Variables|Default|GetGranada))
  (Rendering|SetVisibility _granada _realeasedgranada false)
  (if _realeasedgranada
    (bind _outhit (Class|GameplayStatics|BlueprintPredictProjectilePathbyTraceChannel (Transformation|GetWorldLocation (Variables|Default|GetArrow1)) (* (Math|Vector|GetForwardVector (Pawn|GetControlRotation :!class /Script/Engine.Pawn)) (Variables|Default|GetImpulsoGrana)) true 2e+01 "ECC_WorldDynamic" false 0 "ForOneFrame"))
    (Transformation|SetWorldLocationAndRotation _granada (.ImpactPoint (Collision|BreakHitResult _outhit)) (Math|Rotator|MakeRotfromX (.Normal (Collision|BreakHitResult _outhit))) false false)))

(event Collision|EventActorBeginOverlap
  (params (OtherActor :type Actor%20Object%20Reference)))

(event EventBeginPlay
  ;[1 1 1] Barra de vida
  (Utilities|FlowControl|Sequence
    (:then_0
      ;[1 1 1] Bujula Widget
      (bind _returnvalue (UserInterface|CreateWidget "/Game/Blueprints/Interfaz/Brujula.Brujula_C"))
      (UserInterface|Viewport|AddtoPlayerScreen _returnvalue))
    (:then_1
      (Utilities|FlowControl|Sequence
        (:then_0
          ;[1 1 1] Gravedad 01
          (Utilities|Time|SetTimerbyFunctionName 0 "DireccionGravedad" 0.1 true))
        (:then_1
          (bind _asrem_instance (Utilities|Casting|CastToREM_instance (Game|GetGameInstance)))
          (bind _output_get (Variables|Default|Setinstance%20reference _asrem_instance))
          (if (!= (Variables|/Game/Blueprints/Rem_instance.REM_instance_C|GetlifeInstance _output_get) 0.0)
            (Variables|Default|Setlife (Variables|/Game/Blueprints/Rem_instance.REM_instance_C|GetlifeInstance (Variables|Default|Getinstance%20reference)))
            (else
              (Variables|Default|Setlife 1.0))))))))

(event EventTick
  (params (DeltaSeconds :type Float%20%28single-precision%29))
  ;[1 1 1] Gravedad
  (Utilities|FlowControl|Gate true
    (:Exit
      (Physics|AddForce (Variables|Character|GetCharacterMovement) (Math|Vector|MakeVector 0.0 0.0 (+ (Variables|Default|GetFuerzaGravedad) 1e+05))))))

(event Input|ActionEvents|InputActionCorrer
  (params (Key :type Key%20Structure :default "None"))
  (bind _charactermovement (Variables|Character|GetCharacterMovement))
  ;[1 1 1] movimiento
  (:Pressed
    (Variables|/Script/Engine.CharacterMovementComponent|SetMaxWalkSpeed _charactermovement 3e+02))
  (:Released
    (Variables|/Script/Engine.CharacterMovementComponent|SetMaxWalkSpeed _charactermovement 1.5e+02)))

(event Input|ActionEvents|InputActionDisparo
  (params (Key :type Key%20Structure :default "None"))
  (:Pressed
    (Utilities|FlowControl|FlipFlop
      (:A
        (Rendering|Material|SetScalarParameterValue "/Game/Materiales/Glitch/Pc_Pixel.Pc_Pixel" "Switch" 1.0 :!class /Script/Engine.KismetMaterialLibrary))
      (:B
        (Rendering|Material|SetScalarParameterValue "/Game/Materiales/Glitch/Pc_Pixel.Pc_Pixel" "Switch" 0.0 :!class /Script/Engine.KismetMaterialLibrary :!label _label))))
  (:Released
    (goto _label)))

(event Input|ActionEvents|InputActionPausar
  (params (Key :type Key%20Structure :default "None"))
  (bind _returnvalue (Game|GetPlayerController 0))
  ;[1 1 1] Pausa
  (:Pressed
    (bind _returnvalue_2 (UserInterface|CreateWidget "/Game/Blueprints/Interfaz/Pausa.Pausa_C" _returnvalue))
    (UserInterface|Viewport|AddtoPlayerScreen _returnvalue_2)
    (Input|SetInputModeUIOnly _returnvalue _returnvalue_2 "DoNotLock")
    (Variables|/Script/Engine.PlayerController|SetbShowMouseCursor _returnvalue true)))

(event Input|ActionEvents|InputActionFormateoCamara
  (params (Key :type Key%20Structure :default "None"))
  ;[1 1 1] Formateo de Camara
  (:Pressed
    (Variables|Default|SetCamaraFormateo true)))

(event Input|ActionEvents|InputActionsalto
  (params (Key :type Key%20Structure :default "None"))
  ;[1 1 1] movimiento
  (:Pressed
    (if (Variables|Default|GetCambioGravedad)
      (Character|LaunchCharacter (Math|Vector|MakeVector 0.0 0.0 -7e+02) false false)
      (else
        (Character|Jump)))))

(event Input|ActionEvents|InputActionDisparo
  (params (Key :type Key%20Structure :default "None"))
  (:Pressed
    (bind _outhits (Collision|MultiLineTraceByChannel (+ (Transformation|GetActorLocation) "0, 0,15.000000") (* (Math|Rotator|GetRotationXVector (Transformation|GetActorRotation)) 1.2e+03) "TraceTypeQuery2" false 0 "Persistent"))
    (bind _asdestructible_actor (Utilities|Casting|CastToDestructibleActor (.HitActor (Collision|BreakHitResult (stale _array_element)))))
    (Class|DestructibleComponent|ApplyRadiusDamage (Variables|/Script/ApexDestruction.DestructibleActor|GetDestructibleComponent _asdestructible_actor) 3.5e+02 (.Location (Collision|BreakHitResult (stale _array_element))) 1.0 0.0 false)
    (Effects|SpawnEmitteratLocation 0 (.Location (Collision|BreakHitResult (stale _array_element))) (Math|Rotator|FindLookatRotation (.ImpactPoint (Collision|BreakHitResult (stale _array_element))) (.ImpactNormal (Collision|BreakHitResult (stale _array_element)))))
    (Audio|PlaySoundatLocation "/Game/Sonidos/Waves/Gun/Gun_ShotGun.Gun_ShotGun" (Transformation|GetActorLocation) "0, 0, 0" 1.0 1.0 0.0 0 0 0)))

(event Input|AxisEvents|InputAxisMirar
  (params (AxisValue :type Float%20%28single-precision%29))
  ;[1 1 1] movimiento
  (Pawn|Input|AddControllerPitchInput (Math|Float|SelectFloat (* AxisValue -1.0) AxisValue (Variables|Default|GetCambioGravedad))))

(event Input|AxisEvents|InputAxisRotar
  (params (AxisValue :type Float%20%28single-precision%29))
  ;[1 1 1] movimiento
  (if (not (Variables|Default|GetCamaraFormateo))
    (Pawn|Input|AddControllerYawInput (Math|Float|SelectFloat (* AxisValue -1.0) AxisValue (Variables|Default|GetCambioGravedad)))))

(event Input|AxisEvents|InputAxisDerIzq
  (params (AxisValue :type Float%20%28single-precision%29))
  ;[1 1 1] movimiento
  (Pawn|Input|AddMovementInput (Math|Vector|GetRightVector (Math|Rotator|MakeRotator 0.0 0.0 (.yaw (Pawn|GetControlRotation (Game|GetPlayerController 0) :!class /Script/Engine.Controller)))) (Math|Float|SelectFloat (* AxisValue -1.0) AxisValue (Variables|Default|GetCambioGravedad)) false))

(event Input|AxisEvents|InputAxisAdelanteAtras
  (params (AxisValue :type Float%20%28single-precision%29))
  ;[1 1 1] movimiento
  (Pawn|Input|AddMovementInput (Math|Vector|GetForwardVector (Math|Rotator|MakeRotator 0.0 0.0 (.yaw (Pawn|GetControlRotation (Game|GetPlayerController 0) :!class /Script/Engine.Controller)))) AxisValue false))

(event Input|KeyboardEvents|Q
  (params (Key :type Key%20Structure :default "None"))
  ;[1 1 1] Activacion del Outline
  (:Pressed
    (Rendering|Material|SetVectorParameterValue "/Game/Materiales/Outline/PCOutline.PCOutline" "posicion" (Math|Conversions|ToLinearColor(Vector) (Transformation|GetWorldLocation (Variables|Character|GetMesh))) :!class /Script/Engine.KismetMaterialLibrary)
    (Utilities|FlowControl|FlipFlop
      (:A
        (bind _track (Timeline|Línea%20de%20tiempo_0 Play)
          (:Update
            (Rendering|Material|SetScalarParameterValue "/Game/Materiales/Outline/PCOutline.PCOutline" "Radio" _track :!class /Script/Engine.KismetMaterialLibrary))))
      (:B
        (Timeline|Línea%20de%20tiempo_0 Reverse)))))

(event Input|KeyboardEvents|W
  (params (Key :type Key%20Structure :default "None"))
  ;[1 1 1] movimiento
)

(event Input|KeyboardEvents|E
  (params (Key :type Key%20Structure :default "None"))
  (bind _returnvalue (Transformation|GetActorRotation))
  (bind _cameraplayer (Variables|Default|GetCameraPlayer))
  (bind _returnvalue_2 (Transformation|GetWorldRotation _cameraplayer))
  ;[1 1 1] Gravedad
  (:Pressed
    (Utilities|FlowControl|FlipFlop
      (:A
        (Variables|Default|SetCambioGravedad true)
        (Utilities|FlowControl|Sequence
          (:then_0
            (bind _ejex (Timeline|GiroPersonaje PlayFromStart)
              (:Update
                (Transformation|SetActorRotation (Math|Rotator|MakeRotator _ejex (.pitch _returnvalue) (.yaw _returnvalue)))
                (Transformation|SetWorldRotation _cameraplayer (Math|Rotator|MakeRotator _ejex (.pitch _returnvalue_2) (.yaw _returnvalue_2)) false false))))
          (:then_1
            (Utilities|FlowControl|Gate true) ; enters at Open
          )))
      (:B
        (Variables|Default|SetCambioGravedad false)
        (Utilities|FlowControl|Sequence
          (:then_0
            (Timeline|GiroPersonaje Reverse))
          (:then_1
            (Utilities|FlowControl|Gate true) ; enters at Close
          ))))))

(event Input|MouseEvents|MouseWheelUp
  (params (Key :type Key%20Structure :default "None"))
  (bind _returnvalue (Game|GetPlayerCameraManager 0))
  (bind _returnvalue_2 (Transformation|GetActorLocation _returnvalue))
  ;[1 1 1] Portal
  (:Pressed
    (bind _outactors (Actor|GetAllActorsOfClass "/Game/Blueprints/Portal/Portal_2.Portal_2_C"))
    (Actor|DestroyActor _outactors)
    (bind _outhit (Collision|LineTraceByChannel _returnvalue_2 (+ _returnvalue_2 (* (Transformation|GetActorForwardVector _returnvalue) 5e+03)) "TraceTypeQuery1" false 0 "ForDuration"))
    (bind _returnvalue_3 (Game|SpawnActorfromClass "/Game/Blueprints/Portal/Portal_2.Portal_2_C" (Math|Conversions|ToTransform(Vector) (.Location (Collision|BreakHitResult _outhit))) "Undefined" 0 0))
    (Transformation|SetActorRotation _returnvalue_3 (Math|Rotator|FindLookatRotation (Transformation|GetActorLocation _returnvalue_3) (Transformation|GetActorLocation)))))

(event Input|MouseEvents|RightMouseButton
  (params (Key :type Key%20Structure :default "None"))
  ;[1 1 1] Granada
  (:Pressed
    (Variables|Default|SetRealeasedGranada false)
    (if (Variables|Default|GetRealeasedGranada) :!label _label
      (Variables|Default|SetImpulsoGrana (+ (Variables|Default|GetImpulsoGrana) 1.5e+02))
      (Utilities|FlowControl|Delay 0.2)
      (goto _label)))
  (:Released
    (Variables|Default|SetRealeasedGranada false)
    (Game|SpawnActorfromClass "/Game/Blueprints/MappinGranada/MGranada.MGranada_C" (Math|Transform|MakeTransform (Transformation|GetWorldLocation (Variables|Default|GetArrow1)) (Pawn|GetControlRotation :!class /Script/Engine.Pawn) "1,1,1") "Undefined" 0 (Variables|Default|GetImpulsoGrana) 0)
    (Variables|Default|SetImpulsoGrana 0.0)))

(event Input|MouseEvents|MouseWheelDown
  (params (Key :type Key%20Structure :default "None"))
  (bind _returnvalue (Game|GetPlayerCameraManager 0))
  (bind _returnvalue_2 (Transformation|GetActorLocation _returnvalue))
  ;[1 1 1] Portal
  (:Pressed
    (bind _outactors (Actor|GetAllActorsOfClass "/Game/Blueprints/Portal/Portal_1.Portal_1_C"))
    (Actor|DestroyActor _outactors)
    (bind _outhit (Collision|LineTraceByChannel _returnvalue_2 (+ _returnvalue_2 (* (Transformation|GetActorForwardVector _returnvalue) 5e+03)) "TraceTypeQuery1" false 0 "ForDuration"))
    (bind _returnvalue_3 (Game|SpawnActorfromClass "/Game/Blueprints/Portal/Portal_1.Portal_1_C" (Math|Conversions|ToTransform(Vector) (.Location (Collision|BreakHitResult _outhit))) "Undefined" 0 0))
    (Transformation|SetActorRotation _returnvalue_3 (Math|Rotator|FindLookatRotation (Transformation|GetActorLocation _returnvalue_3) (Transformation|GetActorLocation)))))

(fn ConstructionScript)

(fn DireccionGravedad
  (bind _returnvalue (Transformation|GetActorLocation))
  (bind (_x _y _z) (Math|Vector|BreakVector _returnvalue))
  (bind _returnvalue_2 (Collision|LineTraceForObjects _returnvalue (Math|Vector|MakeVector _x _y (+ _z 1e+02)) (Variables|Default|GetGeneralStaticMesh) false 0 "None"))
  (if _returnvalue_2
    (Variables|Default|SetGravedad true)
    (else
      (Variables|Default|SetGravedad false))))