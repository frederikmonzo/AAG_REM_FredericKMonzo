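; Erick is the player character, with camera-relative movement, jump, sprint and a pause widget that switches input to UI only.
; On BeginPlay it restores Life from the REM game instance, defaulting to full when the stored value is zero.
; Q toggles an outline by writing mesh position and a timeline-driven radius into a Material Parameter Collection.
; Firing runs a debug-drawn multi-trace, sound and emitter, but the hit loop supplying the emitter's location is never executed.
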(event EventBeginPlay
  ;[1 1 1] Barra de vida
  (bind _asrem_instance (Utilities|Casting|CastToREM_instance (Game|GetGameInstance)))
  (bind _output_get (Variables|Default|Setinstance%20reference _asrem_instance))
  (if (!= (Variables|/Game/Blueprints/Rem_instance.REM_instance_C|GetlifeInstance _output_get) 0.0)
    (Variables|Default|Setlife (Variables|/Game/Blueprints/Rem_instance.REM_instance_C|GetlifeInstance (Variables|Default|Getinstance%20reference)))
    (else
      (Variables|Default|Setlife 1.0))))

(event Collision|EventActorBeginOverlap
  (params (OtherActor :type Actor%20Object%20Reference)))

(event Input|ActionEvents|InputActionsalto
  (params (Key :type Key%20Structure :default "None"))
  ;[1 1 1] movimiento
  (:Pressed
    (Character|Jump)))

(event Input|ActionEvents|InputActionCorrer
  (params (Key :type Key%20Structure :default "None"))
  (bind _charactermovement (Variables|Character|GetCharacterMovement))
  (:Pressed
    (Variables|/Script/Engine.CharacterMovementComponent|SetMaxWalkSpeed _charactermovement 3e+02))
  (:Released
    (Variables|/Script/Engine.CharacterMovementComponent|SetMaxWalkSpeed _charactermovement 1.5e+02)))

(event Input|ActionEvents|InputActionDisparo
  (params (Key :type Key%20Structure :default "None"))
  (:Pressed
    (bind _outhits (Collision|MultiLineTraceByChannel (+ (Transformation|GetActorLocation) "0, 0,15.000000") (* (Math|Rotator|GetRotationXVector (Transformation|GetActorRotation)) 1.2e+03) "TraceTypeQuery2" false 0 "Persistent"))
    (Effects|SpawnEmitteratLocation 0 (.Location (Collision|BreakHitResult (stale _array_element))) (Math|Rotator|FindLookatRotation (.ImpactPoint (Collision|BreakHitResult (stale _array_element))) (.ImpactNormal (Collision|BreakHitResult (stale _array_element)))))
    (Audio|PlaySoundatLocation 0 (Transformation|GetActorLocation) "0, 0, 0" 1.0 1.0 0.0 0 0 0)))

(event Input|ActionEvents|InputActionPausar
  (params (Key :type Key%20Structure :default "None"))
  (bind _returnvalue (Game|GetPlayerController 0))
  ;[1 1 1] Pausa
  (:Pressed
    (bind _returnvalue_2 (UserInterface|CreateWidget "/Game/Blueprints/Interfaz/Pausa.Pausa_C" _returnvalue))
    (UserInterface|Viewport|AddtoPlayerScreen _returnvalue_2)
    (Input|SetInputModeUIOnly _returnvalue _returnvalue_2 "DoNotLock")
    (Variables|/Script/Engine.PlayerController|SetbShowMouseCursor _returnvalue true)))

(event Input|AxisEvents|InputAxisadelante
  (params (AxisValue :type Float%20%28single-precision%29))
  (bind _returnvalue (Game|GetPlayerController 0))
  (bind _returnvalue_2 (Pawn|GetControlRotation _returnvalue :!class /Script/Engine.Controller))
  ;[1 1 1] movimiento
  (Pawn|Input|AddMovementInput (Math|Vector|GetForwardVector (Math|Rotator|MakeRotator (.roll _returnvalue_2) 0.0 (.yaw _returnvalue_2))) AxisValue false))

(event Input|AxisEvents|InputAxisderecha
  (params (AxisValue :type Float%20%28single-precision%29))
  (bind _returnvalue (Game|GetPlayerController 0))
  (bind _returnvalue_2 (Pawn|GetControlRotation _returnvalue :!class /Script/Engine.Controller))
  ;[1 1 1] movimiento
  (Pawn|Input|AddMovementInput (Math|Vector|GetRightVector (Math|Rotator|MakeRotator (.roll _returnvalue_2) 0.0 (.yaw _returnvalue_2))) AxisValue false))

(event Input|AxisEvents|InputAxismirar
  (params (AxisValue :type Float%20%28single-precision%29))
  ;[1 1 1] movimiento
  (Pawn|Input|AddControllerPitchInput AxisValue))

(event Input|AxisEvents|InputAxisrotar
  (params (AxisValue :type Float%20%28single-precision%29))
  ;[1 1 1] movimiento
  (Pawn|Input|AddControllerYawInput AxisValue))

(event Input|KeyboardEvents|Q
  (params (Key :type Key%20Structure :default "None"))
  ;[1 1 1] Activacion del Outline
  (:Pressed
    (Rendering|Material|SetVectorParameterValue "/Game/Materiales/Outline/PCOutline.PCOutline" "posicion" (Math|Conversions|ToLinearColor(Vector) (Transformation|GetWorldLocation (Variables|Character|GetMesh))) :!class /Script/Engine.KismetMaterialLibrary)
    (Utilities|FlowControl|FlipFlop
      (:A
        (bind _track (Timeline|Línea%20de%20tiempo_0 Play)
          (:Update
            (Rendering|Material|SetScalarParameterValue "/Game/Materiales/Outline/PCOutline.PCOutline" "Radio" _track :!class /Script/Engine.KismetMaterialLibrary))))
      (:B
        (Timeline|Línea%20de%20tiempo_0 Reverse)))))

(fn ConstructionScript)