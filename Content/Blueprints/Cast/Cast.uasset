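; Proximity turret (Cast) that rises, lights up and fires projectiles at the player entering its attack sphere.
; Any end overlap on the sphere lowers it, dims the light and stops combat.
; A timeline update lerps rotation toward the player and, via a FireRate delay, spawns physics-velocity projectiles with sound.
; MovePosition eases height with a looping lerp and delay, while the construction script sets materials, color and radius.
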(event OnComponentBeginOverlap(Sphere)
  (params (OverlappedComponent :type Primitive%20Component%20Object%20Reference) (OtherActor :type Actor%20Object%20Reference) (OtherComp :type Primitive%20Component%20Object%20Reference) (OtherBodyIndex :type Integer) (bFromSweep :type Boolean) (SweepResult :type Hit%20Result%20Structure%20%28by%20ref%29))
  (if (== OtherActor (Game|GetPlayerCharacter 0))
    (CallFunction|Activate)))

(event OnComponentEndOverlap(Sphere)
  (params (OverlappedComponent :type Primitive%20Component%20Object%20Reference) (OtherActor :type Actor%20Object%20Reference) (OtherComp :type Primitive%20Component%20Object%20Reference) (OtherBodyIndex :type Integer))
  (if (not (== OverlappedComponent (Game|GetPlayerCharacter 0)))
    (CallFunction|Deactivate)))

(event Custom|Activate
  (Utilities|MovePosition "0,0,50.000000"
    (:End
      (CallFunction|UpdateColor (Variables|Tiers|GetDefaultColor) 5e+03)
      (Variables|Default|SetActivated? true)
      (Audio|SpawnSoundatLocation "/Game/Sonidos/Waves/Cast/Boom_040.Boom_040" "0, 0, 0" "0, 0, 0" 1.0 1.0 0.0 0 0)
      (Timeline|CombatTimeLine Play
        (:Update
          (Utilities|FlowControl|Sequence
            (:then_0
              (CallFunction|UpdateRotation))
            (:then_1
              (Utilities|FlowControl|Delay (Variables|Tiers|GetFireRate))
              (if (Variables|Default|GetActivated?)
                (CallFunction|SpawnProyectil)))))))))

(event Custom|Deactivate
  (Utilities|MovePosition "0,0,-50.000000"
    (:End
      (CallFunction|UpdateColor (Variables|Tiers|GetActivateColor) 1e+03)
      (Variables|Default|SetActivated? false)
      (Timeline|CombatTimeLine Stop
        (:Update
          (Utilities|FlowControl|Sequence
            (:then_0
              (CallFunction|UpdateRotation))
            (:then_1
              (Utilities|FlowControl|Delay (Variables|Tiers|GetFireRate))
              (if (Variables|Default|GetActivated?)
                (CallFunction|SpawnProyectil)))))))))

(fn ConstructionScript
  (Rendering|Material|SetMaterial (Variables|Default|GetCast) 0 (Variables|Tiers|GetBodyMaterial))
  (bind _returnvalue (Rendering|Material|CreateDynamicMaterialInstance (Variables|Default|GetGeoSphere) 0 "/Game/Blueprints/Cast/ProximityMaterial.ProximityMaterial" "None" :!class /Script/Engine.PrimitiveComponent))
  (bind _output_get (Variables|Default|SetDinamicMaterial _returnvalue))
  (Rendering|Material|SetVectorParameterValue _output_get "Color" (Variables|Tiers|GetDefaultColor) :!class /Script/Engine.MaterialInstanceDynamic)
  (Rendering|Components|Light|SetLightColor (Variables|Default|GetPointLight) (Variables|Tiers|GetDefaultColor) true)
  (Components|Sphere|SetSphereRadius (Variables|Default|GetSphere) (Variables|Default|GetRadiusAttack) true))

(fn UpdateRotation
  (Transformation|SetWorldRotation (Variables|Default|GetCast) (Math|Rotator|Lerp(Rotator) (Transformation|GetWorldRotation (Variables|Default|GetCast)) (Math|Rotator|FindLookatRotation (Transformation|GetWorldLocation (Variables|Default|GetCast)) (Transformation|GetActorLocation (Game|Player|GetPlayerPawn 0))) 0.5 true) false false))

(fn UpdateColor
  (params (Color :type Linear%20Color%20Structure) (NewIntensity :type Float%20%28single-precision%29))
  (Rendering|Material|SetVectorParameterValue (Variables|Default|GetDinamicMaterial) "Color" Color :!class /Script/Engine.MaterialInstanceDynamic)
  (Rendering|Components|Light|SetLightColor (Variables|Default|GetPointLight) Color true)
  (Rendering|Components|Light|SetIntensity (Variables|Default|GetPointLight) NewIntensity))

(fn SpawnProyectil
  (bind _spawnpoint (Variables|Default|GetSpawnPoint))
  (bind _returnvalue (Transformation|GetWorldTransform _spawnpoint))
  (bind _returnvalue_2 (Game|SpawnActorfromClass "/Game/Blueprints/Cast/proyectil.Proyectil_C" (Math|Transform|MakeTransform (.location _returnvalue) (.rotation _returnvalue) "1,1,1") "Undefined" 0 0))
  (Physics|SetPhysicsLinearVelocity (Variables|/Game/Blueprints/Cast/proyectil.Proyectil_C|GetProyectil _returnvalue_2) (* (Math|Vector|GetUnitDirection(Vector) (Transformation|GetWorldScale (Variables|Default|GetSpawnPoint)) (Transformation|GetActorLocation (Game|GetPlayerCharacter 0))) (Variables|Tiers|GetProyectilSpeed)) false "None")
  (CallFunction|Sound))

(fn Sound
  (Audio|SpawnSoundatLocation "/Game/Sonidos/Waves/Gun/Gun_ShotGun.Gun_ShotGun" (Transformation|GetWorldScale (Variables|Default|GetSpawnPoint)) "0, 0, 0" 1.0 0.5 0.0 0 0))